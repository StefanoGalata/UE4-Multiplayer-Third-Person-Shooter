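; BP_PU_SuperSpeed is a powerup that temporarily doubles the movement speed of the character it activates for.
; On activation it casts the target to Character, stores the reference and doubles that character's MaxWalkSpeed.
; On expiry it halves the current MaxWalkSpeed if the stored character is still valid, rather than restoring a saved value, then calls the parent expiry logic.
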(event `self.OnActivated`
  (params (ActiveFor :type "Actor Object Reference"))
  (bind _ascharacter (cast `Character` ActiveFor))
  (set `self.ActivatedForCharacter` _ascharacter)
  (bind _charactermovement (`Character.CharacterMovement` _ascharacter))
  (set `CharacterMovementComponent.MaxWalkSpeed` (* (`CharacterMovementComponent.MaxWalkSpeed` _charactermovement) 2.0) _charactermovement))

(event `self.OnExpired`
  (bind _activatedforcharacter (`self.ActivatedForCharacter`)
    (:`then`
      (bind _charactermovement (`Character.CharacterMovement` _activatedforcharacter))
      (set `CharacterMovementComponent.MaxWalkSpeed` (/ (`CharacterMovementComponent.MaxWalkSpeed` _charactermovement) 2.0) _charactermovement))
    (:`else`
      _))
  (`parent.OnExpired`))

(fn `UserConstructionScript`)